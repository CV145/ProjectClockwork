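; Candle light prop with a flame particle and a flickering point light.
; The construction script switches between lit and unlit meshes via Enabled and applies intensity, candle material, shadow casting and separate mesh and light mobility.
; On BeginPlay, a timeline at FlickerRate lerps light intensity between min and max.
; Random timeline start times and flame material offsets vary the flicker between instances.
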(event `self.ReceiveBeginPlay`
  ;[1 1 1] Light flicker with random offset
  (`TimelineComponent.SetPlayRate` (`self.Light_Intensity`) (`self.FlickerRate`))
  (`|ExecutionSequence`
    (:`then_0`
      (bind (_direction _intensity) (`Timeline|Light_Intensity` :`NewTime` (`KismetMathLibrary.RandomFloatInRange` 0.0 5.0) :!via `SetNewTime` :!label _label)
        (:`Update`
          (`LightComponent.SetIntensity` (`self.Point Light`) (`KismetMathLibrary.Lerp` (`self.MinIntensity`) (`self.MaxIntensity`) _intensity))
          (`/Engine/EditorBlueprintResources/StandardMacros.DoOnce` false
            (:`Completed`
              (bind _returnvalue (`PrimitiveComponent.CreateDynamicMaterialInstance` (`self.Particle System`) 0 null "None"))
              (`MaterialInstanceDynamic.SetScalarParameterValue` _returnvalue "Offset" (`KismetMathLibrary.RandomFloatInRange` 1.0 2.0)))))))
    (:`then_1`
      (goto _label))))

(fn `UserConstructionScript`
  (bind _castshadow (`self.CastShadow`))
  (bind _enabled (`self.Enabled`))
  (`|ExecutionSequence`
    (:`then_0`
      ;[1 1 1] Toggle light
      (set `self.Enabled` _enabled)
      (`SceneComponent.SetVisibility` (`self.Point Light`) _enabled false)
      (`SceneComponent.SetVisibility` (`self.Particle System`) (`self.Enabled`) false)
      (`SceneComponent.SetVisibility` (`self.SM_Candle`) (not (`self.Enabled`)) false)
      (`SceneComponent.SetVisibility` (`self.SM_Candle_SS`) (`self.Enabled`) false))
    (:`then_1`
      (`LightComponent.SetIntensity` (`self.Point Light`) (`self.Intensity`))
      (bind _returnvalue (`PrimitiveComponent.CreateDynamicMaterialInstance` (`self.Particle System`) 0 null "None"))
      (`MaterialInstanceDynamic.SetScalarParameterValue` _returnvalue "Offset" (`KismetMathLibrary.RandomFloatInRange` 1.0 2.0))
      (`PrimitiveComponent.CreateDynamicMaterialInstance` (`self.SM_Candle_SS`) 0 (`self.CandleMaterial`) "None")
      (`PrimitiveComponent.CreateDynamicMaterialInstance` (`self.SM_Candle`) 0 (`self.CandleMaterial`) "None")
      ;[1 1 1] Cast shadow
      (`|ExecutionSequence`
        (:`then_0`
          (`PrimitiveComponent.SetCastShadow` (`self.SM_Candle`) _castshadow))
        (:`then_1`
          (`PrimitiveComponent.SetCastShadow` (`self.SM_Candle_SS`) _castshadow))))
    (:`then_2`
      ;[1 1 1] Mobility
      (`SceneComponent.SetMobility` (`|MakeArray` (`self.SM_Candle`) (`self.SM_Candle_SS`) :!type "SceneComponent Object Reference") (`self.MeshMobility`))
      (`SceneComponent.SetMobility` (`self.Particle System`) (`self.MeshMobility`))
      (`SceneComponent.SetMobility` (`self.Point Light`) (`self.LightMobility`)))))