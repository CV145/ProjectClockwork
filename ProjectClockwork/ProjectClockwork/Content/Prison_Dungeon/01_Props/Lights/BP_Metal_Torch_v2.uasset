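; BP_Metal_Torch_v2 is a metal torch light prop whose stationary light flickers at runtime.
; The construction script sets the light's base intensity.
; On BeginPlay, a timeline starts at a random time with a configurable play rate, so torches flicker out of sync, and its curve blends the light between minimum and maximum intensity.
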(event `self.ReceiveBeginPlay`
  ;[1 1 1] Light flicker
  (`TimelineComponent.SetPlayRate` (`self.Light_Intensity`) (`self.FlickerRate`))
  (`|ExecutionSequence`
    (:`then_0`
      (bind (_direction _intensity) (`Timeline|Light_Intensity` :`NewTime` (`KismetMathLibrary.RandomFloatInRange` 0.0 5.0) :!via `SetNewTime` :!label _label)
        (:`Update`
          (`LightComponent.SetIntensity` (`self.Stationary Light`) (`KismetMathLibrary.Lerp` (`self.MinIntensity`) (`self.MaxIntensity`) _intensity)))))
    (:`then_1`
      (goto _label))))

(fn `UserConstructionScript`
  (`LightComponent.SetIntensity` (`self.Stationary Light`) (`self.Intensity`)))