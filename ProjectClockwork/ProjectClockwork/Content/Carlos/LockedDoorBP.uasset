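; Locked door actor that an Engineer character can open by spending a key held in the TopDownGameMode.
; Overlapping its box shows a door widget to any PaperCharacter, but enables Interact input only for an Engineer while keys remain; leaving disables it.
; Interact consumes a key, marks the door open and plays a timeline that rotates the door's yaw.
; Doors flagged open at BeginPlay start already rotated.
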(event `self.Box.OnComponentBeginOverlap`
  (params (OverlappedComponent :type "PrimitiveComponent Object Reference") (OtherActor :type "Actor Object Reference") (OtherComp :type "PrimitiveComponent Object Reference") (OtherBodyIndex :type Integer) (bFromSweep :type Boolean) (SweepResult :type "HitResult Structure (by ref)"))
  (if (not (`self.isOpen`))
    (bind _aspaper_character (cast `PaperCharacter` OtherActor))
    (if (`PrimitiveComponent.IsOverlappingActor` (`self.Box`) _aspaper_character)
      (bind _returnvalue (`|CreateWidget` "/Game/Carlos/DoorWidget.DoorWidget_C" null self))
      (`UserWidget.AddToViewport` _returnvalue 0)
      (cast `/Game/0PlayerFinal/Engineer` OtherActor)
      ;[1 1 1] Is door open?
      (if (not (`self.isOpen`))
        (bind _astop_down_game_mode (cast `/Game/TopDownBP/Blueprints/TopDownGameMode` (`GameplayStatics.GetGameMode`)))
        (if (> (`/Game/TopDownBP/Blueprints/TopDownGameMode.keys` _astop_down_game_mode) 0)
          (`self.EnableInput` (`GameplayStatics.GetPlayerController` 0)))))))

(event `self.Box.OnComponentEndOverlap`
  (params (OverlappedComponent :type "PrimitiveComponent Object Reference") (OtherActor :type "Actor Object Reference") (OtherComp :type "PrimitiveComponent Object Reference") (OtherBodyIndex :type Integer))
  (`self.DisableInput` (`GameplayStatics.GetPlayerController` 0)))

(event `InputAction|Interact`
  (params (Key :type "Key Structure"))
  (:`Pressed`
    (bind _astop_down_game_mode (cast `/Game/TopDownBP/Blueprints/TopDownGameMode` (`GameplayStatics.GetGameMode`)))
    (`/Engine/EditorBlueprintResources/StandardMacros.DecrementInt` (`/Game/TopDownBP/Blueprints/TopDownGameMode.keys` _astop_down_game_mode)
      (:`  `
        (set `self.isOpen` true)
        (bind (_direction _floattrack) (`Timeline|OpenDoor` :`NewTime` 2.0) ; Timeline calls code each frame
          (:`Update`
            (`SceneComponent.K2_SetRelativeRotation` (`self.Door`) (`KismetMathLibrary.MakeRotator` 0.0 0.0 _floattrack) false false)))))))

(event `self.ReceiveBeginPlay`
  (if (`self.isOpen`)
    (`SceneComponent.K2_SetRelativeRotation` (`self.Door`) (`KismetMathLibrary.MakeRotator` 0.0 0.0 -180.0) false false)))

(fn `UserConstructionScript`)